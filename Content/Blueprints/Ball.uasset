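; Ball actor for what appears to be a paddle-and-wall game, moving in a random direction on the XZ plane chosen at BeginPlay.
; Tick moves the sphere along that direction at MovementSpeed, using a swept offset.
; Hit events check for Wall or Paddle tags, print debug messages and call Bounce on matches.
; Bounce only draws a debug arrow along the hit trace, leaving the direction unchanged.
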(event `self.ReceiveBeginPlay`
  ;[1 1 1] Randomize starting direction
  (set `self.movementDirection` (`KismetMathLibrary.Normal` (`KismetMathLibrary.MakeVector` (`KismetMathLibrary.RandomFloatInRange` -1.0 1.0) 0.0 (`KismetMathLibrary.RandomFloatInRange` -1.0 1.0)))))

(event `self.ReceiveTick`
  (params (DeltaSeconds :type "Float (single-precision)"))
  ;[1 1 1] Move ball every tick
  (`SceneComponent.K2_AddRelativeLocation` (`self.Sphere`) (* (`self.movementDirection`) (* DeltaSeconds (`self.movementSpeed`))) true false))

(event `self.ReceiveHit`
  (params (MyComp :type "PrimitiveComponent Object Reference") (Other :type "Actor Object Reference") (OtherComp :type "PrimitiveComponent Object Reference") (bSelfMoved :type Boolean) (HitLocation :type "Vector Structure") (HitNormal :type "Vector Structure") (NormalImpulse :type "Vector Structure") (Hit :type "HitResult Structure (by ref)"))
  (bind _tags (`Actor.Tags` Other))
  (if (`KismetArrayLibrary.Array_Contains` _tags "Wall")
    (`KismetSystemLibrary.PrintString` "Ball hit wall" true true (struct :`R` 1.0 :`B` 1.0 :`A` 1.0))
    (`self.Bounce` Hit)
    (elif (`KismetArrayLibrary.Array_Contains` _tags "Paddle")
      (`KismetSystemLibrary.PrintString` "Ball hit paddle" true true (struct :`G` 1.0 :`A` 1.0))
      (`self.Bounce` Hit)
      (else
        (`KismetSystemLibrary.PrintString` "Ball hit something")))))

(fn `Bounce`
  (params (`Hit Data` :type "HitResult Structure"))
  (bind (_bblockinghit _binitialoverlap _time _distance _location _impactpoint _normal _impactnormal _physmat _hitactor _hitcomponent _hitbonename _hititem _faceindex _tracestart _traceend) (`GameplayStatics.BreakHitResult` `Hit Data`))
  (`KismetSystemLibrary.DrawDebugArrow` _tracestart _traceend 50.0 (struct :`R` 1.0 :`A` 1.0) 2.0 2.0)
  (return))

(fn `UserConstructionScript`)