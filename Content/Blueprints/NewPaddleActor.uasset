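; NewPaddleActor is a keyboard-controlled paddle that slides along its local X axis, with key sets for up to two players.
; The construction script sets PlayerID from the count of existing paddle actors and picks arrow keys or A/D for IDs 0 and 1.
; AnyKey events match those keys to set held-direction flags.
; Tick turns the flags into a frame-rate-independent, teleporting offset, with left taking priority over right.
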(event `Key|AnyKey`
  (params (Key :type "Key Structure"))
  (bind _returnvalue (== Key (`self.KeyRight`)))
  (bind _returnvalue_2 (== Key (`self.KeyLeft`)))
  ;[1 0.5042 0.5062] Paddle Input
  (:`Pressed`
    (if _returnvalue_2
      (set `self.LeftDown` true)
      (elif _returnvalue
        (set `self.RightDown` true))))
  (:`Released`
    (if _returnvalue_2
      (set `self.LeftDown` false)
      (elif _returnvalue
        (set `self.RightDown` false)))))

(event `self.ReceiveTick`
  (params (DeltaSeconds :type "Float (single-precision)"))
  ;[1 1 1] Move based on current input
  (if (`self.LeftDown`)
    (set `self.MoveDirection` 1)
    (elif (`self.RightDown`)
      (bind _output_get (set `self.MoveDirection` -1))
      (else
        (set `self.MoveDirection` 0))))
  (if (not (== _output_get 0))
    (`self.K2_AddActorLocalOffset` (`KismetMathLibrary.MakeVector` (* (`self.MoveSpeed`) (`KismetMathLibrary.Conv_IntToDouble` (`self.MoveDirection`)) DeltaSeconds)) false true)))

(fn `UserConstructionScript`
  (bind _outactors (`GameplayStatics.GetAllActorsOfClass` "NewPaddleActor_C"))
  (bind _output_get (set `self.PlayerID` (`KismetArrayLibrary.Array_Length` _outactors)))
  (switch `int` _output_get
    (:`0`
      (set `self.KeyLeft` "Left")
      (set `self.KeyRight` "Right"))
    (:`1`
      (set `self.KeyLeft` "A")
      (set `self.KeyRight` "D"))))